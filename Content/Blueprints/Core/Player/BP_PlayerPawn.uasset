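; BP_PlayerPawn is the player's camera pawn, with panning, spring-arm zoom and stepped rotation.
; Axis inputs shift a desired location along the actor's forward and right vectors and adjust a clamped desired arm length.
; Rotation actions turn the desired rotation in 45-degree steps.
; Tick interpolates location, rotation and arm length toward these targets for smooth camera motion.
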(event EventTick
  (params (DeltaSeconds :type Float%20%28single-precision%29))
  ;[1 1 1] Camera Zoom
  (Variables|/Script/Engine.SpringArmComponent|SetTargetArmLength (Variables|Default|GetSpringArm) (Math|Interpolation|FInterpTo (Variables|/Script/Engine.SpringArmComponent|GetTargetArmLength (Variables|Default|GetSpringArm)) (Variables|Default|GetZoom_Desired) DeltaSeconds 5.0))
  (Transformation|SetActorLocation (Math|Interpolation|VInterpTo (Transformation|GetActorLocation) (Variables|Default|GetLocation_Desired) DeltaSeconds 5.0) false false)
  (Transformation|SetActorRotation (Math|Interpolation|RInterpTo (Transformation|GetActorRotation) (Variables|Default|GetRotation_Desired) DeltaSeconds 1e+01)))

(event EventBeginPlay
  ;[1 0.401 0.401] Event Begin Play
  (Variables|Default|SetLocation_Desired (Transformation|GetActorLocation))
  (Variables|Default|SetZoom_Desired (Variables|/Script/Engine.SpringArmComponent|GetTargetArmLength (Variables|Default|GetSpringArm)))
  (Variables|Default|SetRotation_Desired (Transformation|GetActorRotation)))

(event Input|ActionEvents|InputActionInputAction_RotationLeft
  (params (Key :type Key%20Structure :default "None"))
  ;[0.7216 0.7451 1] Rotate Camera Left
  (:Pressed
    (Variables|Default|SetRotation_Desired (Math|Rotator|CombineRotators (Variables|Default|GetRotation_Desired) "0,45.000000, 0"))))

(event Input|ActionEvents|InputActionInputAction_RotationRight
  (params (Key :type Key%20Structure :default "None"))
  ;[0.7216 0.7451 1] Rotate Camera Right
  (:Pressed
    (Variables|Default|SetRotation_Desired (Math|Rotator|CombineRotators (Variables|Default|GetRotation_Desired) "0,-45.000000, 0"))))

(event Input|AxisEvents|InputAxisInputAxis_Zoom
  (params (AxisValue :type Float%20%28single-precision%29))
  ;[1 1 1] Camera Zoom
  (Variables|Default|SetZoom_Desired (Math|Float|Clamp(Float) (+ (* AxisValue 75.0) (Variables|Default|GetZoom_Desired)) 1e+02 5e+03)))

(event Input|AxisEvents|InputAxisInputAxis_Forward
  (params (AxisValue :type Float%20%28single-precision%29))
  ;[1 0.9647 0.6039] Move Camera Left
  (Variables|Default|SetLocation_Desired (+ (Variables|Default|GetLocation_Desired) (* (Transformation|GetActorForwardVector) (* AxisValue 1e+01)))))

(event Input|AxisEvents|InputAxisInputAxis_Right
  (params (AxisValue :type Float%20%28single-precision%29))
  ;[1 0.9647 0.6039] Move Camera Right
  (Variables|Default|SetLocation_Desired (+ (Variables|Default|GetLocation_Desired) (* (Transformation|GetActorRightVector) (* AxisValue 1e+01)))))

(fn ConstructionScript)